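; Visual control actor for a Mavrik gun controller model, showing button presses, touch feedback and LED states.
; Button events play a press animation and particle effect, then return to the base pose after PressDuration; Trigger also spawns BP_MavrikBullet at the muzzle flash.
; LED events set emissive strength parameters on the mesh materials.
; Touch-area hit events pass stored TouchPositionU/V values to their particle systems before activating them.
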(event OnComponentHit(SM_TouchAreaTop)
  (params (HitComponent :type Primitive%20Component%20Object%20Reference) (OtherActor :type Actor%20Object%20Reference) (OtherComp :type Primitive%20Component%20Object%20Reference) (NormalImpulse :type Vector :default "0, 0, 0") (Hit :type Hit%20Result%20Structure%20%28by%20ref%29))
  (bind _p_touchareatop (Variables|Default|GetP_TouchAreaTop))
  (Effects|Components|ParticleSystem|SetFloatParameter _p_touchareatop "TouchPositionU" (Variables|Default|GetTouchPositionU))
  (Components|Activation|Activate _p_touchareatop true))

(event OnComponentHit(SM_TouchAreaFront)
  (params (HitComponent :type Primitive%20Component%20Object%20Reference) (OtherActor :type Actor%20Object%20Reference) (OtherComp :type Primitive%20Component%20Object%20Reference) (NormalImpulse :type Vector :default "0, 0, 0") (Hit :type Hit%20Result%20Structure%20%28by%20ref%29))
  (bind _p_touchareafront (Variables|Default|GetP_TouchAreaFront))
  (Effects|Components|ParticleSystem|SetFloatParameter _p_touchareafront "TouchPositionU" (Variables|Default|GetTouchPositionU))
  (Components|Activation|Activate _p_touchareafront true))

(event OnComponentHit(SM_TouchAreaBottom)
  (params (HitComponent :type Primitive%20Component%20Object%20Reference) (OtherActor :type Actor%20Object%20Reference) (OtherComp :type Primitive%20Component%20Object%20Reference) (NormalImpulse :type Vector :default "0, 0, 0") (Hit :type Hit%20Result%20Structure%20%28by%20ref%29))
  (bind _p_touchareabottom (Variables|Default|GetP_TouchAreaBottom))
  (Effects|Components|ParticleSystem|SetFloatParameter _p_touchareabottom "TouchPositionU" (Variables|Default|GetTouchPositionU))
  (Components|Activation|Activate _p_touchareabottom true))

(event OnComponentHit(SM_TouchAreaInnerBottom)
  (params (HitComponent :type Primitive%20Component%20Object%20Reference) (OtherActor :type Actor%20Object%20Reference) (OtherComp :type Primitive%20Component%20Object%20Reference) (NormalImpulse :type Vector :default "0, 0, 0") (Hit :type Hit%20Result%20Structure%20%28by%20ref%29))
  (bind _p_touchareainnerbottom (Variables|Default|GetP_TouchAreaInnerBottom))
  (Effects|Components|ParticleSystem|SetFloatParameter _p_touchareainnerbottom "TouchPositionU" (Variables|Default|GetTouchPositionU))
  (Components|Activation|Activate _p_touchareainnerbottom true))

(event OnComponentHit(SM_TouchAreaInnerTop)
  (params (HitComponent :type Primitive%20Component%20Object%20Reference) (OtherActor :type Actor%20Object%20Reference) (OtherComp :type Primitive%20Component%20Object%20Reference) (NormalImpulse :type Vector :default "0, 0, 0") (Hit :type Hit%20Result%20Structure%20%28by%20ref%29))
  (bind _p_touchareainnertop (Variables|Default|GetP_TouchAreaInnerTop))
  (Effects|Components|ParticleSystem|SetFloatParameter _p_touchareainnertop "TouchPositionU" (Variables|Default|GetTouchPositionU))
  (Components|Activation|Activate _p_touchareainnertop true))

(event OnComponentHit(SM_TouchAreaTouchPad)
  (params (HitComponent :type Primitive%20Component%20Object%20Reference) (OtherActor :type Actor%20Object%20Reference) (OtherComp :type Primitive%20Component%20Object%20Reference) (NormalImpulse :type Vector :default "0, 0, 0") (Hit :type Hit%20Result%20Structure%20%28by%20ref%29))
  (bind _p_touchareatouchpadl (Variables|Default|GetP_TouchAreaTouchpadL))
  (Effects|Components|ParticleSystem|SetFloatParameter _p_touchareatouchpadl "TouchPositionU" (Variables|Default|GetTouchPositionU))
  (Effects|Components|ParticleSystem|SetFloatParameter _p_touchareatouchpadl "TouchPositionV" (Variables|Default|GetTouchPositionV))
  (Components|Activation|Activate _p_touchareatouchpadl true))

(event OnComponentHit(SM_TouchAreaTouchPadR)
  (params (HitComponent :type Primitive%20Component%20Object%20Reference) (OtherActor :type Actor%20Object%20Reference) (OtherComp :type Primitive%20Component%20Object%20Reference) (NormalImpulse :type Vector :default "0, 0, 0") (Hit :type Hit%20Result%20Structure%20%28by%20ref%29))
  (bind _p_touchareatouchpadr (Variables|Default|GetP_TouchAreaTouchpadR))
  (Effects|Components|ParticleSystem|SetFloatParameter _p_touchareatouchpadr "TouchPositionU" (Variables|Default|GetTouchPositionU))
  (Effects|Components|ParticleSystem|SetFloatParameter _p_touchareatouchpadr "TouchPositionV" (Variables|Default|GetTouchPositionV))
  (Components|Activation|Activate _p_touchareatouchpadr true))

(event Custom|Trigger
  (Components|Animation|PlayAnimation (Variables|Default|GetMavrik) "/Game/MavrikGun/Animations/A__Armature_Trigger.A__Armature_Trigger" false)
  (Components|Activation|Activate (Variables|Default|GetP_TriggerPress) true)
  (Components|Activation|Activate (Variables|Default|GetP_Mavrik_MuzzleFlash) true)
  (Game|SpawnActorfromClass "/Game/MavrikGun/BP_MavrikBullet.BP_MavrikBullet_C" (Transformation|GetWorldTransform (Variables|Default|GetP_Mavrik_MuzzleFlash)) "Undefined" self 0)
  (Utilities|FlowControl|Delay (Variables|Default|GetPressDuration))
  (Components|Animation|PlayAnimation (Variables|Default|GetMavrik) "/Game/MavrikGun/Animations/A__Armature_Base.A__Armature_Base" false))

(event Custom|TouchLeft
  (Components|Animation|PlayAnimation (Variables|Default|GetMavrik) "/Game/MavrikGun/Animations/A__Armature_TouchLeft.A__Armature_TouchLeft" false)
  (Components|Activation|Activate (Variables|Default|GetP_TouchLPress) true)
  (Utilities|FlowControl|Delay (Variables|Default|GetPressDuration))
  (Components|Animation|PlayAnimation (Variables|Default|GetMavrik) "/Game/MavrikGun/Animations/A__Armature_Base.A__Armature_Base" false))

(event Custom|Left
  (Components|Animation|PlayAnimation (Variables|Default|GetMavrik) "/Game/MavrikGun/Animations/A__Armature_Left.A__Armature_Left" false)
  (Components|Activation|Activate (Variables|Default|GetP_LeftPress) true)
  (Utilities|FlowControl|Delay (Variables|Default|GetPressDuration))
  (Components|Animation|PlayAnimation (Variables|Default|GetMavrik) "/Game/MavrikGun/Animations/A__Armature_Base.A__Armature_Base" false))

(event Custom|LedStripesOn
  (Rendering|Material|SetScalarParameterValueonMaterials (Variables|Default|GetMavrik) "LedStripesStrength" 5.0))

(event Custom|Right
  (Components|Animation|PlayAnimation (Variables|Default|GetMavrik) "/Game/MavrikGun/Animations/A__Armature_Right.A__Armature_Right" false)
  (Components|Activation|Activate (Variables|Default|GetP_RightPress) true)
  (Utilities|FlowControl|Delay (Variables|Default|GetPressDuration))
  (Components|Animation|PlayAnimation (Variables|Default|GetMavrik) "/Game/MavrikGun/Animations/A__Armature_Base.A__Armature_Base" false))

(event Custom|LedStripesOff
  (Rendering|Material|SetScalarParameterValueonMaterials (Variables|Default|GetMavrik) "LedStripesStrength" 0.0))

(event Custom|TouchRight
  (Components|Animation|PlayAnimation (Variables|Default|GetMavrik) "/Game/MavrikGun/Animations/A__Armature_TouchRight.A__Armature_TouchRight" false)
  (Components|Activation|Activate (Variables|Default|GetP_TouchRPress) true)
  (Utilities|FlowControl|Delay (Variables|Default|GetPressDuration))
  (Components|Animation|PlayAnimation (Variables|Default|GetMavrik) "/Game/MavrikGun/Animations/A__Armature_Base.A__Armature_Base" false))

(event Custom|LedHaloOff
  (Rendering|Material|SetScalarParameterValueonMaterials (Variables|Default|GetMavrik) "LedHaloStrength" 0.0))

(event Custom|PowerButton
  (Components|Animation|PlayAnimation (Variables|Default|GetMavrik) "/Game/MavrikGun/Animations/A__Armature_Power.A__Armature_Power" false)
  (Components|Activation|Activate (Variables|Default|GetP_PowerPress) true)
  (Utilities|FlowControl|Delay (Variables|Default|GetPressDuration))
  (Components|Animation|PlayAnimation (Variables|Default|GetMavrik) "/Game/MavrikGun/Animations/A__Armature_Base.A__Armature_Base" false))

(event Custom|LedPowerOff
  (Rendering|Material|SetScalarParameterValueonMaterials (Variables|Default|GetMavrik) "LedPowerStrength" 0.0))

(event Custom|Idle
  (Components|Animation|PlayAnimation (Variables|Default|GetMavrik) "/Game/MavrikGun/Animations/A__Armature_Base.A__Armature_Base" false))

(event Custom|TouchpadsTouch
  (Components|Activation|Activate (Variables|Default|GetP_TouchpadTouch) true))

(event Custom|LedPowerOn
  (Rendering|Material|SetScalarParameterValueonMaterials (Variables|Default|GetMavrik) "LedPowerStrength" 5.0))

(event Custom|FrontTop
  (Components|Animation|PlayAnimation (Variables|Default|GetMavrik) "/Game/MavrikGun/Animations/A__Armature_FrontTop.A__Armature_FrontTop" false)
  (Components|Activation|Activate (Variables|Default|GetP_TopPress) true)
  (Utilities|FlowControl|Delay (Variables|Default|GetPressDuration))
  (Components|Animation|PlayAnimation (Variables|Default|GetMavrik) "/Game/MavrikGun/Animations/A__Armature_Base.A__Armature_Base" false))

(event Custom|LedHaloOn
  (Rendering|Material|SetScalarParameterValueonMaterials (Variables|Default|GetMavrik) "LedHaloStrength" 5.0))

(event Custom|FrontBottom
  (Components|Animation|PlayAnimation (Variables|Default|GetMavrik) "/Game/MavrikGun/Animations/A__Armature_FrontBottom.A__Armature_FrontBottom" false)
  (Components|Activation|Activate (Variables|Default|GetP_BottomPress) true)
  (Utilities|FlowControl|Delay (Variables|Default|GetPressDuration))
  (Components|Animation|PlayAnimation (Variables|Default|GetMavrik) "/Game/MavrikGun/Animations/A__Armature_Base.A__Armature_Base" false))

(event EventBeginPlay
  (CallFunction|Idle))

(fn ConstructionScript)