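; BP_MavrikBullet is a short-lived bullet actor for MavrikClassic that bursts into a hit particle effect and destroys itself.
; Overlap and Hit events share one check that compares the overlap event's OtherActor with the owner, skipping the owner and printing a debug "HIT" otherwise.
; That impact path and a one-second BeginPlay lifetime delay both end in spawning P_MavrikHit at the root's transform and destroying the actor.
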(event EventBeginPlay
  (bind _defaultsceneroot (Variables|Default|GetDefaultSceneRoot))
  (bind _returnvalue (Transformation|GetWorldTransform _defaultsceneroot))
  (bind (_location _rotation) (Math|Transform|BreakTransform _returnvalue))
  (Utilities|FlowControl|Delay 1.0)
  (Effects|SpawnEmitteratLocation "/Game/MavrikGun/VFX/P_MavrikHit.P_MavrikHit" _location _rotation)
  (Actor|DestroyActor))

(event EventTick
  (params (DeltaSeconds :type Float%20%28single-precision%29)))

(event Collision|EventHit
  (params (MyComp :type Primitive%20Component%20Object%20Reference) (Other :type Actor%20Object%20Reference) (OtherComp :type Primitive%20Component%20Object%20Reference) (bSelfMoved :type Boolean) (HitLocation :type Vector :default "0, 0, 0") (HitNormal :type Vector :default "0, 0, 0") (NormalImpulse :type Vector :default "0, 0, 0") (Hit :type Hit%20Result%20Structure%20%28by%20ref%29))
  (bind _defaultsceneroot (Variables|Default|GetDefaultSceneRoot))
  (bind _returnvalue (Transformation|GetWorldTransform _defaultsceneroot))
  (bind (_location _rotation) (Math|Transform|BreakTransform _returnvalue))
  (if (not (== (Components|GetOwner) (stale Collision|EventActorBeginOverlap OtherActor)))
    (Development|PrintString "HIT")
    (Effects|SpawnEmitteratLocation "/Game/MavrikGun/VFX/P_MavrikHit.P_MavrikHit" _location _rotation)
    (Actor|DestroyActor)))

(event Collision|EventActorBeginOverlap
  (params (OtherActor :type Actor%20Object%20Reference))
  (bind _defaultsceneroot (Variables|Default|GetDefaultSceneRoot))
  (bind _returnvalue (Transformation|GetWorldTransform _defaultsceneroot))
  (bind (_location _rotation) (Math|Transform|BreakTransform _returnvalue))
  (if (not (== (Components|GetOwner) OtherActor))
    (Development|PrintString "HIT")
    (Effects|SpawnEmitteratLocation "/Game/MavrikGun/VFX/P_MavrikHit.P_MavrikHit" _location _rotation)
    (Actor|DestroyActor)))

(fn ConstructionScript)