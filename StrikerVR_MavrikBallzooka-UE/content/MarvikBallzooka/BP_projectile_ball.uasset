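; BP_projectile_ball is a ball projectile for the Ballzooka, moved by a ProjectileMovement component.
; The construction script copies the Vel and Speed variables into that component's velocity and initial speed.
; On BeginPlay, the IsSmallBall flag selects a reduced or full-size ball mesh and a matching ribbon width for the Niagara trail.
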(event EventBeginPlay
  (Transformation|SetWorldScale3D (Variables|Default|GetSM_ball) (select (Variables|Default|GetisSmallBall?) "0.400000,0.400000,0.400000" "1.000000,1.000000,1.000000"))
  (Niagara|SetNiagaraVariable(Float) (Variables|Default|GetTrail) "ribbonWidth" (select (Variables|Default|GetisSmallBall?) 2.0 5.0)))

(fn ConstructionScript
  (Variables|/Script/Engine.MovementComponent|SetVelocity (Variables|Default|GetProjectileMovement) (Variables|Default|Getvel))
  (Variables|/Script/Engine.ProjectileMovementComponent|SetInitialSpeed (Variables|Default|GetProjectileMovement) (Variables|Default|Getspeed)))