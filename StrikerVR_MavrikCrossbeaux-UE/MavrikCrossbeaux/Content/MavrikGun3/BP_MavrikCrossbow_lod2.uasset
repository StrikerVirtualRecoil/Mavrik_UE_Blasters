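; Crossbow weapon that fires explosive or rope bullets, driving its animation Blueprint's state, button and loading-progress variables.
; Reload plays a timeline, then spawns the selected bullet on the BulletMount socket.
; Shot detaches the loaded bullet and launches it through its projectile movement, attaching a visible cable to rope bullets.
; Switching ammo toggles the bullet class and respawns any loaded bullet.
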(event Custom|Reload
  (bind _crossbowanimbp (Variables|Default|GetCrossbowAnimBP))
  (if (not (Variables|Default|GetLoaded?))
    (bind _newtrack_0 (Timeline|Loading PlayFromStart)
      (:Update
        (Variables|/Game/MavrikGun3/SkeletalMesh/Crossbow_AnimBlueprint.Crossbow_AnimBlueprint_C|SetLoadingProgress _crossbowanimbp _newtrack_0)
        (Variables|/Game/MavrikGun3/SkeletalMesh/Crossbow_AnimBlueprint.Crossbow_AnimBlueprint_C|SetState _crossbowanimbp "Loading"))
      (:Finished
        (Variables|Default|SetLoaded? true)
        (Variables|/Game/MavrikGun3/SkeletalMesh/Crossbow_AnimBlueprint.Crossbow_AnimBlueprint_C|SetState _crossbowanimbp "Loaded")
        (CallFunction|LoadBullet self)
        (Rendering|SetVisibility (Variables|Default|GetCable) false false)
        (Class|CableComponent|SetAttachEndto (Variables|Default|GetCable) 0 "None" "Capsule")))))

(event Custom|Shot
  (bind _bullet (Variables|Default|GetBullet))
  (Variables|/Game/MavrikGun3/SkeletalMesh/Crossbow_AnimBlueprint.Crossbow_AnimBlueprint_C|SetButtons (Variables|Default|GetCrossbowAnimBP) "Trigger")
  (if (Variables|Default|GetLoaded?)
    (Variables|/Game/MavrikGun3/SkeletalMesh/Crossbow_AnimBlueprint.Crossbow_AnimBlueprint_C|SetState (Variables|Default|GetCrossbowAnimBP) "Shot")
    (Components|Activation|Activate (Variables|Default|GetP_CrossbowTrail) false)
    (Variables|Default|SetLoaded? false)
    (Utilities|FlowControl|Delay 0.1)
    (Transformation|DetachFromComponent (Variables|/Script/Engine.Actor|GetRootComponent _bullet) "KeepWorld" "KeepWorld" "KeepWorld" true)
    (Game|Components|ProjectileMovement|SetVelocityinLocalSpace (Variables|/Game/MavrikGun3/BP_CrossbowBullet.BP_CrossbowBullet_C|GetProjectileMovement1 _bullet) "0.000000, 0,-2000.000000")
    (Variables|/Game/MavrikGun3/SkeletalMesh/Crossbow_AnimBlueprint.Crossbow_AnimBlueprint_C|SetButtons (Variables|Default|GetCrossbowAnimBP) "NotPressed")
    (if (Variables|Default|GetRopeBullet?)
      (Class|CableComponent|SetAttachEndto (Variables|Default|GetCable) (Variables|Default|GetBullet) "None" "Capsule")
      (Rendering|SetVisibility (Variables|Default|GetCable) true false))
    (else
      (Utilities|FlowControl|Delay 0.3)
      (Variables|/Game/MavrikGun3/SkeletalMesh/Crossbow_AnimBlueprint.Crossbow_AnimBlueprint_C|SetButtons (Variables|Default|GetCrossbowAnimBP) "NotPressed"))))

(event Custom|ChangeAmmoType
  (Variables|/Game/MavrikGun3/SkeletalMesh/Crossbow_AnimBlueprint.Crossbow_AnimBlueprint_C|SetButtons (Variables|Default|GetCrossbowAnimBP) "Side")
  (if (Variables|Default|GetRopeBullet?)
    (Variables|Default|SetRopeBullet? false)
    (Variables|Default|SetBulletType "/Game/MavrikGun3/BP_CrossbowBullet_Expl.BP_CrossbowBullet_Expl_C")
    (else
      (Variables|Default|SetRopeBullet? true)
      (Variables|Default|SetBulletType "/Game/MavrikGun3/BP_CrossbowBullet_Rope.BP_CrossbowBullet_Rope_C")))
  (Utilities|FlowControl|Delay 0.2)
  (Variables|/Game/MavrikGun3/SkeletalMesh/Crossbow_AnimBlueprint.Crossbow_AnimBlueprint_C|SetButtons (Variables|Default|GetCrossbowAnimBP) "NotPressed")
  (if (Variables|Default|GetLoaded?)
    (Actor|DestroyActor (Variables|Default|GetBullet))
    (CallFunction|LoadBullet self)))

(event EventBeginPlay
  (bind _ascrossbow_anim_blueprint (Utilities|Casting|CastToCrossbow_AnimBlueprint (Components|SkeletalMesh|GetAnimInstance (Variables|Default|GetSK_MavrikCrossbow)))
    (:then
      (Variables|Default|SetCrossbowAnimBP _ascrossbow_anim_blueprint))
    (:CastFailed
      (Development|PrintString "Cast to AminBP Failed"))))

(fn ConstructionScript)

(fn LoadBullet
  (params (Owner :type Actor%20Object%20Reference))
  (bind _returnvalue (Game|SpawnActorfromClass (Variables|Default|GetBulletType) (Math|Transform|MakeTransform "0, 0,-16.957024" "0,-90.000000, 0") "Undefined" Owner 0))
  (bind _output_get (Variables|Default|SetBullet _returnvalue))
  (Transformation|AttachComponentToComponent _output_get (Variables|Default|GetSK_MavrikCrossbow) "BulletMount" "KeepRelative" "SnapToTarget" "KeepRelative" true))