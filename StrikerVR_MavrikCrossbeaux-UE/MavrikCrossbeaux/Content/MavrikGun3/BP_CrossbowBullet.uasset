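; BP_CrossbowBullet is the crossbow bullet actor, which animates the shape of its mesh as it spawns.
; On BeginPlay, the BulletSpawn timeline plays from the start and drives three morph targets on BulletCrossbow2 from the components of one vector track.
; Each weight is the absolute difference between its component and one, inverting curve values that lie between zero and one.
; The graph contains no movement or hit logic.
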(event Collision|EventActorBeginOverlap
  (params (OtherActor :type Actor%20Object%20Reference)))

(event EventTick
  (params (DeltaSeconds :type Float%20%28single-precision%29)))

(event EventBeginPlay
  (bind _newtrack_1 (Timeline|BulletSpawn PlayFromStart)
    (:Update
      (Components|SkeletalMesh|SetMorphTarget (Variables|Default|GetBulletCrossbow2) "Key 4" (Math|Float|Absolute(Float) (- (.X (Math|Vector|BreakVector _newtrack_1)) 1.0)) false)
      (Components|SkeletalMesh|SetMorphTarget (Variables|Default|GetBulletCrossbow2) "Key 2" (Math|Float|Absolute(Float) (- (.Z (Math|Vector|BreakVector _newtrack_1)) 1.0)) false)
      (Components|SkeletalMesh|SetMorphTarget (Variables|Default|GetBulletCrossbow2) "Key 1" (Math|Float|Absolute(Float) (- (.Y (Math|Vector|BreakVector _newtrack_1)) 1.0)) false))))

(fn ConstructionScript)